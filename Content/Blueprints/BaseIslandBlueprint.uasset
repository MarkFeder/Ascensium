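; Base island Blueprint that procedurally assembles a randomized island from four copies of one model mesh in its construction script.
; It first gives its existing static mesh components random meshes from the obstacle list.
; It then offsets each copy to a corner derived from the model's bounds, with a random yaw from a preset angle list.
; Each obstacle component snaps to its portion's "Obstacle" socket.
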(fn `GetRandomAngle`
  (returns (float :type "Float (double-precision)"))
  (bind _randomangles (`self.RandomAngles`))
  (return (`KismetArrayLibrary.Array_Get` _randomangles (`KismetMathLibrary.RandomInteger` (`KismetArrayLibrary.Array_Length` _randomangles)))))

(fn `SetupMeshComponents`
  (params (StaticMeshes :type "Array of StaticMesh Object Reference"))
  (for _array_element (`self.K2_GetComponentsByClass` "/Script/Engine.StaticMeshComponent")
    (`StaticMeshComponent.SetStaticMesh` _array_element (`KismetArrayLibrary.Array_Get` StaticMeshes (`KismetMathLibrary.RandomInteger` (`KismetArrayLibrary.Array_Length` StaticMeshes))))))

(fn `UserConstructionScript`
  (bind (_origin _boxextent) (`KismetMathLibrary.BreakBoxSphereBounds` (`StaticMesh.GetBounds` (`self.ModelMesh`))))
  (bind _x (.x _boxextent))
  (bind _y (.y _boxextent))
  ;[1 1 1] Get Root location
  (set `self.PosXModelMesh` (.x (`SceneComponent.K2_GetComponentLocation` (`self.DefaultSceneRoot`))))
  (set `self.PosYModelMesh` (.y (`SceneComponent.K2_GetComponentLocation` (`self.DefaultSceneRoot`))))
  (set `self.PosZModelMesh` (.z (`SceneComponent.K2_GetComponentLocation` (`self.DefaultSceneRoot`))))
  (`self.SetupMeshComponents` (`self.ObstacleStaticMeshes`))
  (`KismetSystemLibrary.PrintString` (`KismetStringLibrary.Conv_VectorToString` _origin) true true (struct :`R` 0.605 :`G` 0.0121 :`B` 0.026077 :`A` 1.0) 5.0)
  (`KismetSystemLibrary.PrintString` (`KismetStringLibrary.Conv_VectorToString` _boxextent) true true (struct :`G` 0.66 :`B` 1.0 :`A` 1.0) 5.0)
  ;[0.9918 1 0.39] Generate pos values in which the different portions should be placed
  (set `self.Point01Pos` (`KismetMathLibrary.MakeVector` (* _x -1.0) (* _y -1.0)))
  (set `self.Point02Pos` (`KismetMathLibrary.MakeVector` _x _y))
  (set `self.Point03Pos` (`KismetMathLibrary.MakeVector` _x (* _y -1.0)))
  (set `self.Point04Pos` (`KismetMathLibrary.MakeVector` (* _x -1.0) _y))
  ;[1 1 1] Setup random angles
  (bind _float (`self.GetRandomAngle`))
  (bind _float_2 (`self.GetRandomAngle`))
  (bind _float_3 (`self.GetRandomAngle`))
  (bind _float_4 (`self.GetRandomAngle`))
  (`|ExecutionSequence`
    (:`then_0`
      ;[1 0.405 0.4813] Generate portion meshes
      (bind _returnvalue (`AddComponent|NODE_AddStaticMeshComponent-4` :`RelativeTransform` (`KismetMathLibrary.MakeTransform` (`self.Point01Pos`) (`KismetMathLibrary.MakeRotator` 0.0 0.0 _float_4) (1.0 1.0 1.0))))
      (`StaticMeshComponent.SetStaticMesh` _returnvalue (`self.ModelMesh`))
      ;[1 1 1] Attach obstacle to the mesh component
      (`SceneComponent.K2_AttachToComponent` (`self.ObstacleMeshComponent01`) _returnvalue "Obstacle" "SnapToTarget" "SnapToTarget" "KeepRelative" true))
    (:`then_1`
      (bind _returnvalue_2 (`AddComponent|NODE_AddStaticMeshComponent-5` :`RelativeTransform` (`KismetMathLibrary.MakeTransform` (`self.Point02Pos`) (`KismetMathLibrary.MakeRotator` 0.0 0.0 _float_3))))
      (`StaticMeshComponent.SetStaticMesh` _returnvalue_2 (`self.ModelMesh`))
      (`SceneComponent.K2_AttachToComponent` (`self.ObstacleMeshComponent02`) _returnvalue_2 "Obstacle" "SnapToTarget" "SnapToTarget" "KeepRelative" true))
    (:`then_2`
      (bind _returnvalue_3 (`AddComponent|NODE_AddStaticMeshComponent-6` :`RelativeTransform` (`KismetMathLibrary.MakeTransform` (`self.Point03Pos`) (`KismetMathLibrary.MakeRotator` 0.0 0.0 _float_2))))
      (`StaticMeshComponent.SetStaticMesh` _returnvalue_3 (`self.ModelMesh`))
      (`SceneComponent.K2_AttachToComponent` (`self.ObstacleMeshComponent03`) _returnvalue_3 "Obstacle" "SnapToTarget" "SnapToTarget" "KeepRelative" true))
    (:`then_3`
      (bind _returnvalue_4 (`AddComponent|NODE_AddStaticMeshComponent-7` :`RelativeTransform` (`KismetMathLibrary.MakeTransform` (`self.Point04Pos`) (`KismetMathLibrary.MakeRotator` 0.0 0.0 _float))))
      (`StaticMeshComponent.SetStaticMesh` _returnvalue_4 (`self.ModelMesh`))
      (`SceneComponent.K2_AttachToComponent` (`self.ObstacleMeshComponent04`) _returnvalue_4 "Obstacle" "SnapToTarget" "SnapToTarget" "KeepRelative" true))))