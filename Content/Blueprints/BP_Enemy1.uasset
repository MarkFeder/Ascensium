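; BP_Enemy1 is an enemy pawn that chases the first-person player and damages them on contact.
; Every tick it issues an AI move toward the cached player reference, re-fetching it if invalid.
; Incoming damage lowers its health, and at zero or below it adds points to the game mode's score, destroys itself and asks the game mode to check remaining enemies.
; Health, point value and contact damage are set in the construction script.
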(event `self.ReceiveBeginPlay`
  (bind _asfirst_person_character_2 (cast `/Game/FirstPersonBP/Blueprints/FirstPersonCharacter_2` (`GameplayStatics.GetPlayerCharacter` 0)))
  (set `self.Player` _asfirst_person_character_2))

(event `self.ReceiveTick`
  (params (DeltaSeconds :type "Float (single-precision)"))
  (bind _player (`self.Player`))
  (`/Engine/EditorBlueprintResources/StandardMacros.IsValid` _player
    (:`Is Valid`
      (`|AIMoveTo` self (0.0 0.0 0.0) _player 16.0))
    (:`Is Not Valid`
      (bind _asfirst_person_character_2 (cast `/Game/FirstPersonBP/Blueprints/FirstPersonCharacter_2` (`GameplayStatics.GetPlayerCharacter` 0)))
      (bind _output_get (set `self.Player` _asfirst_person_character_2))
      (`|AIMoveTo` self (0.0 0.0 0.0) _output_get 16.0))))

(event `ReceiveDamage`
  (params (Damage :type Integer))
  (`self.SetHealth` Damage)
  (bind _enemydead (`self.CheckIsDied`))
  (if _enemydead
    (bind _asfirst_person_game_mode (cast `/Game/FirstPersonBP/Blueprints/FirstPersonGameMode` (`GameplayStatics.GetGameMode`)))
    (`/Game/FirstPersonBP/Blueprints/FirstPersonGameMode.AddPointsToScore` _asfirst_person_game_mode (`self.ValuePoints`))
    (`self.K2_DestroyActor`)
    (`/Game/FirstPersonBP/Blueprints/FirstPersonGameMode.CheckEnemies` _asfirst_person_game_mode)))

(event `self.ReceiveHit`
  (params (MyComp :type "PrimitiveComponent Object Reference") (Other :type "Actor Object Reference") (OtherComp :type "PrimitiveComponent Object Reference") (bSelfMoved :type Boolean) (HitLocation :type "Vector Structure") (HitNormal :type "Vector Structure") (NormalImpulse :type "Vector Structure") (Hit :type "HitResult Structure (by ref)"))
  (bind _asfirst_person_character_2 (cast `/Game/FirstPersonBP/Blueprints/FirstPersonCharacter_2` Other))
  (`/Game/FirstPersonBP/Blueprints/FirstPersonCharacter_2.ReceiveDamage` _asfirst_person_character_2 (`self.ValueDamage`)))

(event `self.ReceiveEndPlay`
  (params (EndPlayReason :type "EEndPlayReason Enum" :default "Destroyed")))

(fn `CheckIsDied`
  (returns (EnemyDead :type Boolean))
  (`/Engine/EditorBlueprintResources/StandardMacros.CompareInt` (`self.Health`)
    (:`>`
      (return false))
    (:`==`
      _)
    (:`<`
      _))
  (return true))

(fn `SetHealth`
  (params (Damage :type Integer))
  (set `self.Health` (- (`self.Health`) Damage)))

(fn `UserConstructionScript`
  (set `self.Health` 2)
  (set `self.ValuePoints` 5)
  (set `self.ValueDamage` 5))