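; Level status Blueprint that tracks a countdown timer and an enemy count for each level, reporting to FirstPersonGameMode.
; Tick decrements CurrentTime while the level runs, but calls GameOver only if it exceeds MAXTime, not at zero.
; CheckEnemies increments the count and calls CanGoNextLevel at MAXEnemies; StartNewLevel also calls it, passing a fixed transform.
; ResetLevel pauses the timer, sets new limits and zeroes both counters.
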(event `self.ReceiveBeginPlay`
  (`self.StartNewLevel`))

(event `self.ReceiveTick`
  (params (DeltaSeconds :type "Float (single-precision)"))
  (if (not (`self.NextLevel`))
    (`/Engine/EditorBlueprintResources/StandardMacros.CompareFloat` (`self.CurrentTime`) (`self.MAXTime`)
      (:`>`
        (bind _asfirst_person_game_mode (cast `/Game/FirstPersonBP/Blueprints/FirstPersonGameMode` (`GameplayStatics.GetGameMode`)))
        (`/Game/FirstPersonBP/Blueprints/FirstPersonGameMode.GameOver` _asfirst_person_game_mode))
      (:`==`
        (`self.SetCurrentTime` DeltaSeconds :!label _label))
      (:`<`
        (goto _label)))))

(event `CheckEnemies`
  (bind _num (`self.SetNumEnemies`))
  (if (== _num (`self.MAXEnemies`))
    (bind _asfirst_person_game_mode (cast `/Game/FirstPersonBP/Blueprints/FirstPersonGameMode` (`GameplayStatics.GetGameMode`)))
    (`/Game/FirstPersonBP/Blueprints/FirstPersonGameMode.CanGoNextLevel` :`self` _asfirst_person_game_mode)))

(event `ResetLevel`
  (params (Time :type "Float (double-precision)") (Enemies :type Integer))
  (set `self.NextLevel` true)
  (set `self.MAXTime` Time)
  (set `self.CurrentTime` 0.0)
  (set `self.NumEnemies` 0)
  (set `self.MAXEnemies` Enemies))

(event `StartNewLevel`
  (set `self.NextLevel` false)
  (bind _asfirst_person_game_mode (cast `/Game/FirstPersonBP/Blueprints/FirstPersonGameMode` (`GameplayStatics.GetGameMode`)))
  ;[1 1 1] Should we store spawn transform to modify next islands
  (`/Game/FirstPersonBP/Blueprints/FirstPersonGameMode.CanGoNextLevel` _asfirst_person_game_mode (`KismetMathLibrary.MakeTransform` (0.0 0.0 200.0))))

(fn `SetCurrentTime`
  (params (DeltaSeconds :type "Float (double-precision)"))
  (returns (Time :type "Float (double-precision)"))
  (bind _output_get (set `self.CurrentTime` (- (`self.CurrentTime`) DeltaSeconds)))
  (`/Engine/EditorBlueprintResources/StandardMacros.CompareFloat` _output_get
    (:`>`
      _)
    (:`==`
      _)
    (:`<`
      (return 0.0)))
  (return _output_get))

(fn `SetNumEnemies`
  (returns (Num :type Integer))
  (bind _output_get (set `self.NumEnemies` (+ (`self.NumEnemies`) 1)))
  (return _output_get))

(fn `UserConstructionScript`
  (bind _output_get (set `self.MAXTime` 300.0))
  (set `self.CurrentTime` _output_get)
  (set `self.MAXEnemies` 10)
  (set `self.NumEnemies` 0)
  (set `self.NextLevel` false))