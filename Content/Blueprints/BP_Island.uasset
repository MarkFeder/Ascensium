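; BP_Island procedurally builds an island from four random portion meshes.
; GenerateIsland offsets each portion into a quadrant by its bounds, adds it with a random yaw, and returns socket world transforms.
; GetSocketLocations passes socket name "None" for portions three and four, unlike the first two.
; The construction script is empty, and helpers for filling sockets with meshes or actors sit outside the generation chain.
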(fn `GenerateIsland`
  (params (PortionMeshes :type "Array of StaticMesh Object Reference"))
  (returns (SpawnTransforms :type "Array of Transform Structure"))
  (set `self.PosXModelMesh` (.x (`SceneComponent.K2_GetComponentLocation` (`self.DefaultSceneRoot`))))
  (set `self.PosYModelMesh` (.y (`SceneComponent.K2_GetComponentLocation` (`self.DefaultSceneRoot`))))
  (set `self.PosZModelMesh` (.z (`SceneComponent.K2_GetComponentLocation` (`self.DefaultSceneRoot`))))
  ;[1 1 1] Get Random Portion Mesh and Setup Variables
  (bind _randommesh (`self.GetRandomPortionMesh` PortionMeshes))
  (bind _output_get (set `self.RandomPortionMesh01` _randommesh))
  (bind _randommesh_2 (`self.GetRandomPortionMesh` PortionMeshes))
  (bind _output_get_2 (set `self.RandomPortionMesh02` _randommesh_2))
  (bind _randommesh_3 (`self.GetRandomPortionMesh` PortionMeshes))
  (bind _output_get_3 (set `self.RandomPortionMesh03` _randommesh_3))
  (bind _randommesh_4 (`self.GetRandomPortionMesh` PortionMeshes))
  (bind _output_get_4 (set `self.RandomPortionMesh04` _randommesh_4))
  (`self.GeneratePointPositions` _output_get _output_get_2 _output_get_3 _output_get_4)
  (bind (_attachedportionmeshcomponent01 _attachedportionmeshcomponent02 _attachedportionmeshcomponent03 _attachedportionmeshcomponent04) (`self.GeneratePortionsMeshComponentsAndAttachTheirStaticMeshes`))
  (bind _socketofmeshcomponentstransforms (`self.GetSocketLocations` _attachedportionmeshcomponent01 _attachedportionmeshcomponent02 _attachedportionmeshcomponent03 _attachedportionmeshcomponent04))
  (return _socketofmeshcomponentstransforms))

(fn `GeneratePointPositions`
  (params (PortionMesh01 :type "StaticMesh Object Reference") (PortionMesh02 :type "StaticMesh Object Reference") (PortionMesh03 :type "StaticMesh Object Reference") (PortionMesh04 :type "StaticMesh Object Reference"))
  ;[0.9918 1 0.39] Generate pos values in which the different portions should be placed
  (set `self.Point01Pos` (`KismetMathLibrary.MakeVector` (* (.x (`.BoxExtent` (`KismetMathLibrary.BreakBoxSphereBounds` (`StaticMesh.GetBounds` PortionMesh01)))) -1.0) (* (.y (`.BoxExtent` (`KismetMathLibrary.BreakBoxSphereBounds` (`StaticMesh.GetBounds` PortionMesh01)))) -1.0)))
  (set `self.Point02Pos` (`KismetMathLibrary.MakeVector` (.x (`.BoxExtent` (`KismetMathLibrary.BreakBoxSphereBounds` (`StaticMesh.GetBounds` PortionMesh02)))) (.y (`.BoxExtent` (`KismetMathLibrary.BreakBoxSphereBounds` (`StaticMesh.GetBounds` PortionMesh02))))))
  (set `self.Point03Pos` (`KismetMathLibrary.MakeVector` (.x (`.BoxExtent` (`KismetMathLibrary.BreakBoxSphereBounds` (`StaticMesh.GetBounds` PortionMesh03)))) (* (.y (`.BoxExtent` (`KismetMathLibrary.BreakBoxSphereBounds` (`StaticMesh.GetBounds` PortionMesh03)))) -1.0)))
  (set `self.Point04Pos` (`KismetMathLibrary.MakeVector` (* (.x (`.BoxExtent` (`KismetMathLibrary.BreakBoxSphereBounds` (`StaticMesh.GetBounds` PortionMesh04)))) -1.0) (.y (`.BoxExtent` (`KismetMathLibrary.BreakBoxSphereBounds` (`StaticMesh.GetBounds` PortionMesh04))))))
  (return))

(fn `GeneratePortionsMeshComponentsAndAttachTheirStaticMeshes`
  (returns (AttachedPortionMeshComponent01 :type "StaticMeshComponent Object Reference") (AttachedPortionMeshComponent02 :type "StaticMeshComponent Object Reference") (AttachedPortionMeshComponent03 :type "StaticMeshComponent Object Reference") (AttachedPortionMeshComponent04 :type "StaticMeshComponent Object Reference"))
  ;[1 1 1] Get random angles
  (bind _float (`self.GetRandomAngle`))
  (bind _float_2 (`self.GetRandomAngle`))
  (bind _float_3 (`self.GetRandomAngle`))
  (bind _float_4 (`self.GetRandomAngle`))
  (`|ExecutionSequence`
    (:`then_0`
      ;[1 1 1] Generate static mesh components and set its static mesh
      (bind _returnvalue (`AddComponent|NODE_AddStaticMeshComponent-18` :`RelativeTransform` (`KismetMathLibrary.MakeTransform` (`self.Point01Pos`) (`KismetMathLibrary.MakeRotator` 0.0 0.0 _float_4))))
      (`StaticMeshComponent.SetStaticMesh` _returnvalue (`self.RandomPortionMesh01`)))
    (:`then_1`
      (bind _returnvalue_2 (`AddComponent|NODE_AddStaticMeshComponent-22` :`RelativeTransform` (`KismetMathLibrary.MakeTransform` (`self.Point02Pos`) (`KismetMathLibrary.MakeRotator` 0.0 0.0 _float_3))))
      (`StaticMeshComponent.SetStaticMesh` _returnvalue_2 (`self.RandomPortionMesh02`)))
    (:`then_2`
      (bind _returnvalue_3 (`AddComponent|NODE_AddStaticMeshComponent-23` :`RelativeTransform` (`KismetMathLibrary.MakeTransform` (`self.Point03Pos`) (`KismetMathLibrary.MakeRotator` 0.0 0.0 _float_2))))
      (`StaticMeshComponent.SetStaticMesh` _returnvalue_3 (`self.RandomPortionMesh03`)))
    (:`then_3`
      (bind _returnvalue_4 (`AddComponent|NODE_AddStaticMeshComponent-24` :`RelativeTransform` (`KismetMathLibrary.MakeTransform` (`self.Point04Pos`) (`KismetMathLibrary.MakeRotator` 0.0 0.0 _float))))
      (`StaticMeshComponent.SetStaticMesh` _returnvalue_4 (`self.RandomPortionMesh04`)))
    (:`then_4`
      (return _returnvalue _returnvalue_2 _returnvalue_3 _returnvalue_4))))

(fn `GetRandomActor`
  (params (Actors :type "Array of Actor Object Reference"))
  (returns (Actor :type "Actor Object Reference"))
  (return (`KismetArrayLibrary.Array_Get` Actors (`KismetMathLibrary.RandomInteger` (`KismetArrayLibrary.Array_Length` Actors)))))

(fn `GetRandomAngle`
  (returns (float :type "Float (double-precision)"))
  (bind _randomangles (`self.RandomAngles`))
  (return (`KismetArrayLibrary.Array_Get` _randomangles (`KismetMathLibrary.RandomInteger` (`KismetArrayLibrary.Array_Length` _randomangles)))))

(fn `GetRandomPortionMesh`
  (params (StaticMeshes :type "Array of StaticMesh Object Reference"))
  (returns (RandomMesh :type "StaticMesh Object Reference"))
  (return (`KismetArrayLibrary.Array_Get` StaticMeshes (`KismetMathLibrary.RandomInteger` (`KismetArrayLibrary.Array_Length` StaticMeshes)))))

(fn `GetRandomStaticMesh`
  (params (StaticMeshes :type "Array of StaticMesh Object Reference"))
  (returns (ObstacleMesh :type "StaticMesh Object Reference"))
  (return (`KismetArrayLibrary.Array_Get` StaticMeshes (`KismetMathLibrary.RandomInteger` (`KismetArrayLibrary.Array_Length` StaticMeshes)))))

(fn `GetSocketLocations`
  (params (AttachedPortionMeshComponent01 :type "StaticMeshComponent Object Reference") (AttachedPortionMeshComponent02 :type "StaticMeshComponent Object Reference") (AttachedPortionMeshComponent03 :type "StaticMeshComponent Object Reference") (AttachedPortionMeshComponent04 :type "StaticMeshComponent Object Reference"))
  (returns (SocketOfMeshComponentsTransforms :type "Array of Transform Structure"))
  (locals (SocketTransforms :type "Array of Transform Structure"))
  (`|ExecutionSequence`
    (:`then_0`
      (for _array_element (`SceneComponent.GetAllSocketNames` AttachedPortionMeshComponent01)
        (`KismetArrayLibrary.Array_Add` (`local.SocketTransforms`) (`SceneComponent.GetSocketTransform` AttachedPortionMeshComponent01 _array_element "RTS_World"))))
    (:`then_1`
      (for _array_element_2 (`SceneComponent.GetAllSocketNames` AttachedPortionMeshComponent02)
        (`KismetArrayLibrary.Array_Add` (`local.SocketTransforms`) (`SceneComponent.GetSocketTransform` AttachedPortionMeshComponent02 _array_element_2 "RTS_World"))))
    (:`then_2`
      (for _ (`SceneComponent.GetAllSocketNames` AttachedPortionMeshComponent03)
        (`KismetArrayLibrary.Array_Add` (`local.SocketTransforms`) (`SceneComponent.GetSocketTransform` AttachedPortionMeshComponent03 "None" "RTS_World"))))
    (:`then_3`
      (for _ (`SceneComponent.GetAllSocketNames` AttachedPortionMeshComponent04)
        (`KismetArrayLibrary.Array_Add` (`local.SocketTransforms`) (`SceneComponent.GetSocketTransform` AttachedPortionMeshComponent04 "None" "RTS_World"))))
    (:`then_4`
      (return (`local.SocketTransforms`)))))

(fn `PopulateSocketsOfStaticMeshComponents`
  (params (AttachedPortionMeshComponent01 :type "StaticMeshComponent Object Reference") (AttachedPortionMeshComponent02 :type "StaticMeshComponent Object Reference") (AttachedPortionMeshComponent03 :type "StaticMeshComponent Object Reference") (AttachedPortionMeshComponent04 :type "StaticMeshComponent Object Reference") (ObstacleMesh :type "Array of StaticMesh Object Reference"))
  ;[1 1 1] For each socket of each portion of the island, attach a new mesh component, set its static mesh and attach it to the original portion
  (`|ExecutionSequence`
    (:`then_0`
      (for _array_element (`SceneComponent.GetAllSocketNames` AttachedPortionMeshComponent01)
        (bind _obstaclemesh (`self.GetRandomStaticMesh` ObstacleMesh))
        (bind _returnvalue (`AddComponent|NODE_AddStaticMeshComponent-25`))
        (`StaticMeshComponent.SetStaticMesh` _returnvalue _obstaclemesh)
        (`SceneComponent.K2_AttachToComponent` _returnvalue AttachedPortionMeshComponent01 _array_element "SnapToTarget" "SnapToTarget" "KeepRelative" true)))
    (:`then_1`
      (for _array_element_2 (`SceneComponent.GetAllSocketNames` AttachedPortionMeshComponent02)
        (bind _obstaclemesh_2 (`self.GetRandomStaticMesh` ObstacleMesh))
        (bind _returnvalue_2 (`AddComponent|NODE_AddStaticMeshComponent-26`))
        (`StaticMeshComponent.SetStaticMesh` _returnvalue_2 _obstaclemesh_2)
        (`SceneComponent.K2_AttachToComponent` _returnvalue_2 AttachedPortionMeshComponent02 _array_element_2 "SnapToTarget" "SnapToTarget" "KeepRelative" true)))
    (:`then_2`
      (for _array_element_3 (`SceneComponent.GetAllSocketNames` AttachedPortionMeshComponent03)
        (bind _obstaclemesh_3 (`self.GetRandomStaticMesh` ObstacleMesh))
        (bind _returnvalue_3 (`AddComponent|NODE_AddStaticMeshComponent-27`))
        (`StaticMeshComponent.SetStaticMesh` _returnvalue_3 _obstaclemesh_3)
        (`SceneComponent.K2_AttachToComponent` _returnvalue_3 AttachedPortionMeshComponent03 _array_element_3 "SnapToTarget" "SnapToTarget" "KeepRelative" true)))
    (:`then_3`
      (for _array_element_4 (`SceneComponent.GetAllSocketNames` AttachedPortionMeshComponent04)
        (bind _obstaclemesh_4 (`self.GetRandomStaticMesh` ObstacleMesh))
        (bind _returnvalue_4 (`AddComponent|NODE_AddStaticMeshComponent-28`))
        (`StaticMeshComponent.SetStaticMesh` _returnvalue_4 _obstaclemesh_4)
        (`SceneComponent.K2_AttachToComponent` _returnvalue_4 AttachedPortionMeshComponent04 _array_element_4 "SnapToTarget" "SnapToTarget" "KeepRelative" true)))))

(fn `SetupMeshComponents`
  (params (StaticMeshes :type "Array of StaticMesh Object Reference"))
  (for _array_element (`self.K2_GetComponentsByClass` "/Script/Engine.StaticMeshComponent")
    (`StaticMeshComponent.SetStaticMesh` _array_element (`KismetArrayLibrary.Array_Get` StaticMeshes (`KismetMathLibrary.RandomInteger` (`KismetArrayLibrary.Array_Length` StaticMeshes))))))

(fn `SpawnActorsOnMeshComponentsSockets`
  (params (AttachedPortionMeshComponent01 :type "StaticMeshComponent Object Reference") (AttachedPortionMeshComponent02 :type "StaticMeshComponent Object Reference") (AttachedPortionMeshComponent03 :type "StaticMeshComponent Object Reference") (AttachedPortionMeshComponent04 :type "StaticMeshComponent Object Reference") (ActorClass :type "Actor Class Reference"))
  (returns (ActorsOnLevel :type "Array of Actor Object Reference"))
  (locals (ArrayOfActors :type "Array of Actor Object Reference"))
  (`|ExecutionSequence`
    (:`then_0`
      (for _array_element (`SceneComponent.GetAllSocketNames` AttachedPortionMeshComponent01)
        (bind _returnvalue (`|SpawnActorFromClass` ActorClass (`KismetMathLibrary.MakeTransform` (`SceneComponent.GetSocketLocation` AttachedPortionMeshComponent01 _array_element)) "Undefined" "OverrideRootScale"))
        (`KismetArrayLibrary.Array_Add` (`local.ArrayOfActors`) _returnvalue)))
    (:`then_1`
      (for _array_element_2 (`SceneComponent.GetAllSocketNames` AttachedPortionMeshComponent02)
        (bind _returnvalue_2 (`|SpawnActorFromClass` ActorClass (`KismetMathLibrary.MakeTransform` (`SceneComponent.GetSocketLocation` AttachedPortionMeshComponent02 _array_element_2)) "Undefined" "OverrideRootScale"))
        (`KismetArrayLibrary.Array_Add` (`local.ArrayOfActors`) _returnvalue_2)))
    (:`then_2`
      (for _array_element_3 (`SceneComponent.GetAllSocketNames` AttachedPortionMeshComponent03)
        (bind _returnvalue_3 (`|SpawnActorFromClass` ActorClass (`KismetMathLibrary.MakeTransform` (`SceneComponent.GetSocketLocation` AttachedPortionMeshComponent03 _array_element_3)) "Undefined" "OverrideRootScale"))
        (`KismetArrayLibrary.Array_Add` (`local.ArrayOfActors`) _returnvalue_3)))
    (:`then_3`
      (for _array_element_4 (`SceneComponent.GetAllSocketNames` AttachedPortionMeshComponent04)
        (bind _returnvalue_4 (`|SpawnActorFromClass` ActorClass (`KismetMathLibrary.MakeTransform` (`SceneComponent.GetSocketLocation` AttachedPortionMeshComponent04 _array_element_4)) "Undefined" "OverrideRootScale"))
        (`KismetArrayLibrary.Array_Add` (`local.ArrayOfActors`) _returnvalue_4)))
    (:`then_4`
      (return (`local.ArrayOfActors`)))))

(fn `UserConstructionScript`
  ;[1 1 1] Get Root location
)