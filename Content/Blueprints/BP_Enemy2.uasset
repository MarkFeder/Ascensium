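; BP_Enemy2 is an enemy that wanders between random navigable points and awards score when killed.
; Each Tick traces forward: an initial overlap prints a hit FirstPersonCharacter's name, otherwise AI MoveTo continues, picking a new point on success.
; Damage lowers Health; at zero or below it adds ValuePoints through FirstPersonGameMode and destroys itself.
; Hitting the player calls their ReceiveDamage with zero damage.
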(event `self.ReceiveBeginPlay`
  (set `self.Destination` (`NavigationSystem.GetRandomPointInNavigableRadius` (`self.K2_GetActorLocation`) 5000.0)))

(event `self.ReceiveTick`
  (params (DeltaSeconds :type "Float (single-precision)"))
  (bind _returnvalue (`self.K2_GetActorLocation`))
  (bind _outhit (`KismetSystemLibrary.LineTraceSingle` :`Start` _returnvalue :`End` (+ _returnvalue (* (`KismetMathLibrary.GetForwardVector` (`self.K2_GetActorRotation`)) 500)) :`TraceChannel` "TraceTypeQuery1" :`DrawDebugType` "Persistent"))
  (bind (_bblockinghit _binitialoverlap _time _location _impactpoint _normal _impactnormal _physmat _hitactor) (`GameplayStatics.BreakHitResult` _outhit))
  (if _binitialoverlap
    (bind _asfirst_person_character (cast `/Game/FirstPersonBP/Blueprints/FirstPersonCharacter` _hitactor))
    (`KismetSystemLibrary.PrintString` (`KismetSystemLibrary.GetDisplayName` _asfirst_person_character))
    (else
      (`|AIMoveTo` self (`self.Destination`)
        (:`OnSuccess`
          (`KismetSystemLibrary.PrintString` "Success")
          (set `self.Destination` (`NavigationSystem.GetRandomPointInNavigableRadius` (`self.K2_GetActorLocation`) 10000.0)))))))

(event `ReceiveDamage`
  (params (Damage :type Integer))
  (bind _valuepoints (`self.ValuePoints`))
  (`self.SetHealth` Damage)
  (bind _enemydead (`self.CheckIsDied`))
  (if _enemydead
    (bind _asfirst_person_game_mode (cast `/Game/FirstPersonBP/Blueprints/FirstPersonGameMode` (`GameplayStatics.GetGameMode`)))
    (`/Game/FirstPersonBP/Blueprints/FirstPersonGameMode.AddPointsToScore` _asfirst_person_game_mode _valuepoints)
    (`KismetSystemLibrary.PrintString` (`KismetStringLibrary.Concat_StrStr` "Points added: " (`KismetStringLibrary.Conv_IntToString` _valuepoints)))
    (`self.K2_DestroyActor`)))

(event `self.ReceiveHit`
  (params (MyComp :type "PrimitiveComponent Object Reference") (Other :type "Actor Object Reference") (OtherComp :type "PrimitiveComponent Object Reference") (bSelfMoved :type Boolean) (HitLocation :type "Vector Structure") (HitNormal :type "Vector Structure") (NormalImpulse :type "Vector Structure") (Hit :type "HitResult Structure (by ref)"))
  (bind _asfirst_person_character (cast `/Game/FirstPersonBP/Blueprints/FirstPersonCharacter` Other))
  (`/Game/FirstPersonBP/Blueprints/FirstPersonCharacter.ReceiveDamage` _asfirst_person_character 0))

(fn `CheckIsDied`
  (returns (EnemyDead :type Boolean))
  (`/Engine/EditorBlueprintResources/StandardMacros.CompareInt` (`self.Health`)
    (:`>`
      (return false))
    (:`==`
      _)
    (:`<`
      _))
  (return true))

(fn `SetHealth`
  (params (Damage :type Integer))
  (set `self.Health` (- (`self.Health`) Damage)))

(fn `UserConstructionScript`
  (set `self.Health` 4)
  (set `self.ValuePoints` 10))